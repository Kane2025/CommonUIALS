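; Main menu camera actor that flies its camera along a spline path on a continuous loop.
; BeginPlay snaps the camera component onto the spline.
; BeginCameraMovement plays a timeline scaled by PlayLength, moving the camera to the spline's world transform at the timeline's alpha and restarting from the start when it finishes.
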(event `self.ReceiveBeginPlay`
  (`SceneComponent.K2_AttachToComponent` (`self.CameraComponent`) (`self.Spline`) "None" "SnapToTarget" "SnapToTarget" "SnapToTarget" true))

(event `Begin Camera Movement`
  (`TimelineComponent.SetPlayRate` (`self.Camera Movement`) (/ 1.0 (`self.Play Length`)))
  (bind (_direction _alpha) (`Timeline|Camera Movement` :!via `PlayFromStart`)
    (:`Update`
      (`SceneComponent.K2_SetWorldTransform` (`self.CameraComponent`) (`SplineComponent.GetTransformAtTime` (`self.Spline`) _alpha "World" false false) false true))
    (:`Finished`
      (`TimelineComponent.PlayFromStart` (`self.Camera Movement`)))))

(fn `UserConstructionScript`)