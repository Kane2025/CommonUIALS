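; BI_HUD is a Blueprint Interface through which other objects reach the game's HUD and its menus.
; It declares getters for the game layer, game menu and menu stacks, the modal queue and the overlay menu.
; It also declares display and remove calls for the main menu, in-game main menu, black screen, and quit and abandon-changes prompts, with active-state queries for all but the black screen and a confirm call for abandoning changes.
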(fn `Confirm Abandon Changes Prompt`)

(fn `Display Abandon Changes Prompt`)

(fn `Display Black Screen`)

(fn `Display In Game Main Menu`)

(fn `Display Main Menu`)

(fn `Display Quit Game Prompt`)

(fn `Get Game Layer Stack`
  (returns (`Game Layer Stack` :type "CommonActivatableWidgetStack Object Reference"))
  (return null))

(fn `Get Game Menu Stack`
  (returns (`Game Menu Stack` :type "CommonActivatableWidgetStack Object Reference"))
  (return null))

(fn `Get Menu Stack`
  (returns (`Get Menu Stack` :type "CommonActivatableWidgetStack Object Reference"))
  (return null))

(fn `Get Modal Queue`
  (returns (`Get Modal Queue` :type "CommonActivatableWidgetQueue Object Reference"))
  (return null))

(fn `Get Overlay Menu`
  (returns (`Overlay Menu` :type "/ALS/ALSExtras/UI/W_OverlayModeMenu Object Reference"))
  (return null))

(fn `Is Abandon Changes Prompt Active`
  (returns (Active :type Boolean))
  (return false))

(fn `Is In Game Main Menu Active`
  (returns (Active :type Boolean))
  (return false))

(fn `Is Main Menu Active`
  (returns (Active :type Boolean))
  (return false))

(fn `Is Quit Game Prompt Active`
  (returns (Active :type Boolean))
  (return false))

(fn `Remove Abandon Changes Prompt`)

(fn `Remove Black Screen`)

(fn `Remove In Game Main Menu`)

(fn `Remove Main Menu`)

(fn `Remove Quit Game Prompt`)