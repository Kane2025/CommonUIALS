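; Main menu player controller that plays startup slides, then shows the menu over rotating camera views with music.
; BeginPlay raises a black screen, sets up Enhanced Input, and polls until the HUD's layer stack is valid.
; Slides advance through finished callbacks; with none configured, it goes straight to cameras and music without calling the HUD's menu display.
; A self-restarting timeline cycles tagged B_MainMenuCamera actors, blending the view target to each.
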(event `Transition To Camera Rotation`
  (message `/Game/Blueprints/Interfaces/BI_HUD.Remove Black Screen` (`self.GetHUD`))
  (`self.Rotate Camera`)
  (message `/Game/Blueprints/Interfaces/BI_HUD.Display Main Menu` (`self.GetHUD`))
  (bind _aseos_game_instance (cast `/Game/UI/CommonUI/EOS_GameInstance` (`GameplayStatics.GetGameInstance`)))
  (`/Game/UI/CommonUI/EOS_GameInstance.Start Main Menu Music` _aseos_game_instance))

(event `self.ReceiveBeginPlay`
  (bind _returnvalue (subsystem `EnhancedInputLocalPlayerSubsystem`))
  (`|ExecutionSequence`
    (:`then_0`
      (message `/Game/Blueprints/Interfaces/BI_HUD.Display Black Screen` (`self.GetHUD`)))
    (:`then_1`
      (message `/Game/Blueprints/Interfaces/BI_GameInstance.Set Instance State` (`GameplayStatics.GetGameInstance`) "NewEnumerator1")
      (if (`self.IsLocalController`)
        (`EnhancedInputSubsystemInterface.RemoveMappingContext` _returnvalue "/ALS/ALS/Data/Input/IMC_Default.IMC_Default" (struct))
        (`EnhancedInputSubsystemInterface.AddMappingContext` _returnvalue "/ALSXT/ALS/Data/Input/IMC_ALSXT_Default.IMC_ALSXT_Default" 0 (struct))
        (bind _returnvalue_2 (`AddComponent|NODE_AddGameplayTasksComponent-0`))
        (set `self.Gameplay Tasks Component` _returnvalue_2)
        (`WidgetBlueprintLibrary.SetFocusToGameViewport`)
        (set `self.bShowMouseCursor` false)))
    (:`then_2`
      (`self.Wait for Primary Layout Readiness` :!label _label
        (:`Ready`
          (if (`KismetArrayLibrary.Array_IsNotEmpty` (`self.Main Menu Startup Slide Array`))
            (`self.Advance Main Menu Slides`)
            (else
              (message `/Game/Blueprints/Interfaces/BI_HUD.Remove Black Screen` (`self.GetHUD`))
              (set `self.bShowMouseCursor` true)
              (`self.Rotate Camera`)
              (bind _aseos_game_instance (cast `/Game/UI/CommonUI/EOS_GameInstance` (`GameplayStatics.GetGameInstance`)))
              (`/Game/UI/CommonUI/EOS_GameInstance.Start Main Menu Music` _aseos_game_instance))))
        (:`Not Ready`
          (`KismetSystemLibrary.Delay` 0.001)
          (goto _label))))))

(event `Rotate Camera`
  (bind _returnvalue (+ (`self.Current Camera Index`) 1))
  (bind _outactors (`GameplayStatics.GetAllActorsOfClassWithTag` "/Game/Blueprints/Cameras/B_MainMenuCamera.B_MainMenuCamera_C" "Main Menu"))
  (bind _output_get (set `self.Camera Array` _outactors))
  (`TimelineComponent.SetPlayRate` (`self.Camera Rotation`) (/ 1.0 (`self.Camera Rotation Time Length`)))
  (bind _debug_mode (message `/Game/Blueprints/Interfaces/BI_GameInstance.Get Debug Mode` (`GameplayStatics.GetGameInstance`)))
  (bind _output (`|GetArrayItem` _output_get (`self.Current Camera Index`)))
  (if (`TimelineComponent.IsPlaying` (`/Game/Blueprints/Cameras/B_MainMenuCamera.Camera Movement` _output))
    (`Timeline|Camera Rotation` :!via `PlayFromStart` :!label _label_2
      (:`Update`
        (`self.SetViewTargetWithBlend` _output 0.75 "VTBlend_EaseInOut" 0.5))
      (:`Finished`
        (set `self.Current Camera Index` (select `bool` (> _returnvalue (`KismetArrayLibrary.Array_LastIndex` (`self.Camera Array`))) :`false` _returnvalue))
        (`self.Rotate Camera`)))
    (else
      (`/Game/Blueprints/Cameras/B_MainMenuCamera.Begin Camera Movement` _output)
      (goto _label_2 :!via `PlayFromStart`))))

(event `On Slide Finished`
  (bind _returnvalue (+ (`self.Main Menu Slide Index`) 1))
  (bind _debug_mode (message `/Game/Blueprints/Interfaces/BI_GameInstance.Get Debug Mode` (`GameplayStatics.GetGameInstance`)))
  (if (> _returnvalue (`KismetArrayLibrary.Array_LastIndex` (`self.Main Menu Startup Slide Array`)))
    (`self.Transition To Camera Rotation`)
    (else
      (set `self.Main Menu Slide Index` _returnvalue)
      (`self.Advance Main Menu Slides`)
      (`CommonActivatableWidget.DeactivateWidget` (stale `Advance Main Menu Slides` _ascbw_slide)))))

(event `Advance Main Menu Slides`
  (bind _get_menu_stack (message `/Game/Blueprints/Interfaces/BI_HUD.Get Menu Stack` (`self.GetHUD`)))
  (bind _returnvalue (`CommonActivatableWidgetContainerBase.BP_AddWidget` _get_menu_stack (`|GetArrayItem` (`self.Main Menu Startup Slide Array`) (`self.Main Menu Slide Index`))))
  (set `self.bShowMouseCursor` false)
  (`KismetSystemLibrary.Delay` 0.3)
  (bind _ascbw_slide (cast `/Game/UI/Widgets/MainMenu/CBW_Slide` _returnvalue))
  (`Widget.SetFocus` _ascbw_slide)
  (`Widget.SetKeyboardFocus` _ascbw_slide)
  (`WidgetBlueprintLibrary.SetInputMode_UIOnlyEx` self _ascbw_slide)
  (add `/Game/UI/Widgets/MainMenu/CBW_Slide.On Finished` _ascbw_slide (delegate `On Slide Finished`)))

(fn `SetGlobalTimeDilation`
  (params (`Time Dilation` :type "Float (double-precision)"))
  (if (`KismetSystemLibrary.IsStandalone`)
    (`GameplayStatics.SetGlobalTimeDilation` (`local.Time Dilation`))))

(fn `UserConstructionScript`)